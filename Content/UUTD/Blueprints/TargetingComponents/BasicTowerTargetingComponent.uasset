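; Targeting component for a tower defense tower that finds the enemies within its aggro radius.
; On BeginPlay it caches its owning TDbasictower.
; Each CheckForTarget call runs a sphere overlap at the tower's FakeOriginPosition, filtered to BasicEnemy actors, and writes the de-duplicated list to the tower's MostRecentTargets.
; It only gathers candidates, with no prioritization, and nothing in this graph triggers the check.
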(event Custom|CheckForTarget
  (Utilities|Array|Clear (Variables|Default|GetTemporaryEnemiesArray)) ; Clear the array that keeps track of recent targets
  (bind _astdbasictower (Utilities|Casting|CastToTDbasictower (Components|GetOwner))
    (:then
      (bind _outactors (Class|KismetSystemLibrary|SphereOverlapActorsNEW (Variables|/Game/UUTD/Blueprints/Towers/TDbasictower.TDbasictower_C|GetFakeOriginPosition _astdbasictower) (Variables|Default|GetAgroRadius) (Utilities|Array|MakeArray "ObjectTypeQuery7") "/Game/UUTD/Blueprints/Enemies/BasicEnemy.BasicEnemy_C")) ; Looks for all actors of type BasicEnemy around tower
      (for _array_element _outactors ; Convert each BasicEnemy into the right class so we can work on it properly.
        (Utilities|Array|AddUnique (Variables|Default|GetTemporaryEnemiesArray) (.AsBasic%20Enemy (Utilities|Casting|CastToBasicEnemy _array_element))))
      (Variables|/Game/UUTD/Blueprints/Towers/TDbasictower.TDbasictower_C|SetMostRecentTargets (Variables|Default|GetOwningTower) (Variables|Default|GetTemporaryEnemiesArray)) ; Send the finished array to the tower we belong to
    )
    (:CastFailed
      (Development|PrintString "TowerAIComponet Not attatched to tower!" true true "(R=1.000000,G=0.000000,B=0.087629,A=1.000000)" 3.0))))

(event EventBeginPlay
  ;[1 1 1] BeginPlay
  (bind _astdbasictower (Utilities|Casting|CastToTDbasictower (Components|GetOwner)))
  (Variables|Default|SetOwningTower _astdbasictower) ; Caches reference to the tower this component is attatched to so that we aren't asking for it every frame
)